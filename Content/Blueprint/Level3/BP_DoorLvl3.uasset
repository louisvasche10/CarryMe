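; BP_DoorLvl3 is a double wooden door for Level 3.
; The OpenDoorLvl3 event opens it if IsLock is true, playing an unlock sound after a short delay.
; If not locked, a BP_FirstPersonLvl3 overlapping the Box triggers a French on-screen message, then opens it after a delay.
; Both paths set ShouldGetOpen, letting Tick rotate both leaves toward their open angles with RInterpTo.
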(event OnComponentBeginOverlap(Box)
  (params (OverlappedComponent :type Primitive%20Component%20Object%20Reference) (OtherActor :type Actor%20Object%20Reference) (OtherComp :type Primitive%20Component%20Object%20Reference) (OtherBodyIndex :type Integer) (bFromSweep :type Boolean) (SweepResult :type Hit%20Result%20Structure%20%28by%20ref%29))
  ;[0.15 0.15 0.15 0.5] La porte s'ouvre
  (Utilities|Casting|CastToBP_FirstPersonLvl3 OtherActor)
  (if (not (Variables|Default|GetbIsLock))
    (Development|PrintString "Boss vous auriez du ouvrir la porte au départ... bon je vous l'ouvre" true true "(R=0.000000,G=0.660000,B=1.000000,A=1.000000)" 3.0)
    (Utilities|FlowControl|Delay 3.0)
    (Variables|Default|SetShouldGetOpen? true)))

(event Custom|OpenDoorLvl3
  ;[0.15 0.15 0.15 0.5] La porte s'ouvre
  (if (== (Variables|Default|GetbIsLock) true)
    (Variables|Default|SetShouldGetOpen? true)
    (Utilities|FlowControl|Delay 0.2)
    (Audio|PlaySound2D "/Game/Feedback/SoundEffect/SoundLevel1/SW_Porte_qui_se_déverouille.SW_Porte_qui_se_déverouille" 1.0 1.0 0.0 0 0)))

(event EventTick
  (params (DeltaSeconds :type Float%20%28single-precision%29))
  (bind _sm_door_wood_left (Variables|Components|GetSM_door_wood_left))
  (bind _sm_door_wood_right (Variables|Components|GetSM_door_wood_right))
  ;[0.15 0.15 0.15 0.5] La porte s'ouvre
  (if (== (Variables|Default|GetShouldGetOpen?) true)
    (Transformation|SetRelativeRotation _sm_door_wood_left (Math|Interpolation|RInterpTo (Variables|/Script/Engine.SceneComponent|GetRelativeRotation _sm_door_wood_left) (Math|Rotator|MakeRotator 0.0 0.0 (Variables|Default|GetOpenAngleL)) DeltaSeconds (Variables|Default|GetOpenSeed)) false false)
    (Transformation|SetRelativeRotation _sm_door_wood_right (Math|Interpolation|RInterpTo (Variables|/Script/Engine.SceneComponent|GetRelativeRotation _sm_door_wood_right) (Math|Rotator|MakeRotator 0.0 0.0 (Variables|Default|GetOpenAngleR)) DeltaSeconds (Variables|Default|GetOpenSeed)) false false)))

(fn ConstructionScript)