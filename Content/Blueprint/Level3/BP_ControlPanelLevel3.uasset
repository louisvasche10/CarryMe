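; Level 3 control panel that lets the player open a linked door with the interact input.
; Overlapping the green trigger, or starting inside it, flags the player as near and is never cleared here.
; Interact always plays a click, but only when near does a timeline lerp the button down, then open LinkedDoor and hide the E prompt.
; The E prompt starts visible and X hidden, with events to show either.
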(event OnComponentBeginOverlap(TriggerGreen)
  (params (OverlappedComponent :type Primitive%20Component%20Object%20Reference) (OtherActor :type Actor%20Object%20Reference) (OtherComp :type Primitive%20Component%20Object%20Reference) (OtherBodyIndex :type Integer) (bFromSweep :type Boolean) (SweepResult :type Hit%20Result%20Structure%20%28by%20ref%29))
  ;[0.15 0.15 0.15 0.5] le panel que le joueur est là donc le rend accessible
  (Utilities|Casting|CastToBP_FirstPersonCharacter OtherActor)
  (Variables|Default|SetRefHero 0)
  (Variables|Default|SetNearPanel true)
  (Rendering|SetVisibility (Variables|Default|GetHintWidget) true false))

(event Custom|ShowX
  ;[0.15 0.15 0.15 0.5] le widget x apparait
  (Rendering|SetVisibility (Variables|Default|GetWidgetX) true true))

(event Custom|ShowE
  ;[0.15 0.15 0.15 0.5] le widget e apparait
  (Rendering|SetVisibility (Variables|Default|GetWidgetE) true true))

(event Custom|ByeE
  ;[0.15 0.15 0.15 0.5] ByeE
  (Rendering|SetVisibility (Variables|Default|GetWidgetE) false true))

(event Input|EnhancedActionEvents|EnhancedInputActionIA_Interact
  (params (ActionValue :type Boolean) (ElapsedSeconds :type Float%20%28double-precision%29) (TriggeredSeconds :type Float%20%28double-precision%29) (InputAction :type Input%20Action%20Object%20Reference :default "/Game/Input/Actions/IA_Interact.IA_Interact"))
  ;[0.15 0.15 0.15 0.5] appuyez sur E pour ouvrir la porte
  (Audio|PlaySound2D "/Game/Feedback/SoundEffect/ClickBouton.ClickBouton" 1.0 1.0 0.0 0 0)
  (if (Variables|Default|GetNearPanel)
    (bind _press (Timeline|Timeline PlayFromStart)
      (:Update
        (Transformation|SetRelativeLocation (Variables|Default|Getbtn) (Math|Vector|Lerp(Vector) (Variables|Default|GetBtn_EStartLocation) (+ (Variables|Default|GetBtn_EStartLocation) "-0.000000,0.000000,-8.000000") _press) false false))
      (:Finished
        (Default|OpenDoorLvl3 (Variables|Default|GetLinkedDoor))
        (CallFunction|ByeE)))))

(event EventBeginPlay
  ;[0.15 0.15 0.15 0.5] les deux widgets sont invisibles au début
  (Variables|Default|SetBtn_XStartLocation (Variables|/Script/Engine.SceneComponent|GetRelativeRotation (Variables|Default|Getlevier)))
  (Variables|Default|SetBtn_EStartLocation (Variables|/Script/Engine.SceneComponent|GetRelativeLocation (Variables|Default|Getbtn)))
  (Rendering|SetVisibility (Variables|Default|GetWidgetE) true true)
  (Rendering|SetVisibility (Variables|Default|GetWidgetX) false true)
  (for _array_element (Collision|GetOverlappingActors (Variables|Default|GetTriggerGreen) "/Game/FirstPerson/Blueprints/BP_FirstPersonCharacter.BP_FirstPersonCharacter_C" :!class /Script/Engine.PrimitiveComponent)
    (Utilities|Casting|CastToBP_FirstPersonCharacter (Game|GetPlayerCharacter 0))
    (Variables|Default|SetNearPanel true)))

(fn ConstructionScript)