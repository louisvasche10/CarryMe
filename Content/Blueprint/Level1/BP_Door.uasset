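; BP_Door is a double wooden door in Level1 that swings open when OpenDoor is called.
; OpenDoor sets IsLock, which despite its name acts as an "opening" flag for Tick.
; Tick eases both leaves' relative rotation toward their open angles with RInterpTo, then clears the flag once both yaws are nearly there.
; The DoorOpen? event is empty, and a timeline animation and hero animation check remain unconnected.
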(event Custom|DoorOpen?
  ;[0.15 0.15 0.15 0.5] Animation de l'ouverture
)

(event EventTick
  (params (DeltaSeconds :type Float%20%28single-precision%29))
  (bind _sm_door_wood_left (Variables|Default|GetSM_door_wood_left))
  (bind _sm_door_wood_right (Variables|Default|GetSM_door_wood_right))
  ;[0.15 0.15 0.15 0.5] La porte s'ouvre
  (if (== (Variables|Default|GetbIsLock) true)
    (Transformation|SetRelativeRotation _sm_door_wood_left (Math|Interpolation|RInterpTo (Variables|/Script/Engine.SceneComponent|GetRelativeRotation _sm_door_wood_left) (Math|Rotator|MakeRotator 0.0 0.0 (Variables|Default|GetOpenAngleL)) DeltaSeconds (Variables|Default|GetOpenSeed)) false false)
    (Transformation|SetRelativeRotation _sm_door_wood_right (Math|Interpolation|RInterpTo (Variables|/Script/Engine.SceneComponent|GetRelativeRotation _sm_door_wood_right) (Math|Rotator|MakeRotator 0.0 0.0 (Variables|Default|GetOpenAngleR)) DeltaSeconds (Variables|Default|GetOpenSeed)) false false)
    (if (and (Math|Float|NearlyEqual(Float) (.Yaw (Math|Rotator|BreakRotator (Variables|/Script/Engine.SceneComponent|GetRelativeRotation _sm_door_wood_left))) (Variables|Default|GetOpenAngleL) 1.0) (Math|Float|NearlyEqual(Float) (.Yaw (Math|Rotator|BreakRotator (Variables|/Script/Engine.SceneComponent|GetRelativeRotation _sm_door_wood_right))) (Variables|Default|GetOpenAngleR) 1.0))
      (Variables|Default|SetbIsLock false))))

(fn ConstructionScript)

(fn OpenDoor
  (Variables|Default|SetbIsLock true))