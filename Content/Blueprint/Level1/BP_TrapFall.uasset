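; BP_TrapFall is a Level 1 floor trap that drops the hero into a hole and teleports them back.
; ActivateTrapFall saves the linked hero's location, disables mesh collision and moves the mesh along Z with a Timeline.
; The Timeline plays a falling sound, waits, then reverses to restore query-only collision and re-arm the trap.
; Hero overlap with BC_SpawnFall triggers a delayed teleport to the saved location, guarded by a respawn flag.
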(event OnComponentBeginOverlap(BC_SpawnFall)
  (params (OverlappedComponent :type Primitive%20Component%20Object%20Reference) (OtherActor :type Actor%20Object%20Reference) (OtherComp :type Primitive%20Component%20Object%20Reference) (OtherBodyIndex :type Integer) (bFromSweep :type Boolean) (SweepResult :type Hit%20Result%20Structure%20%28by%20ref%29))
  ;[0.15 0.15 0.15 0.5] Héro, reapparait + audio de quand il tombe
  (if (not (Variables|Default|GetbIsRespawningHero))
    (Variables|Default|SetbIsRespawningHero true)
    (Utilities|Casting|CastToBP_Hero OtherActor)
    (Utilities|FlowControl|Delay 3.5)
    (Transformation|SetActorLocation (Variables|Default|GetLinkedHero) (Variables|Default|GetHeroSpawnLocation) false true)
    (Variables|Default|SetbIsRespawningHero false)))

(event Custom|ActivateTrapFall
  (bind _staticmesh (Variables|Default|GetStaticMesh))
  (bind _initialmeshlocation (Variables|Default|GetInitialMeshLocation))
  ;[0.15 0.15 0.15 0.5] Comment
  (if (not (Variables|Default|GetTrapAlreadyActivated))
    (Variables|Default|SetHeroSpawnLocation (Transformation|GetActorLocation (Variables|Default|GetLinkedHero)))
    (Collision|SetCollisionEnabled (Variables|Default|GetStaticMesh) "NoCollision")
    (Variables|Default|SetTrapAlreadyActivated true)
    (bind (_direction _trapfall) (Timeline|Timeline Play)
      (:Update
        (Transformation|SetRelativeLocation _staticmesh (Math|Vector|MakeVector (.x _initialmeshlocation) (.y _initialmeshlocation) _trapfall) false false))
      (:Finished
        (if (== _direction 0)
          (Audio|PlaySound2D "/Game/Feedback/SoundEffect/SoundLevel1/SW_HeroFallingInHoleLvl1.SW_HeroFallingInHoleLvl1" 1.0 1.0 0.0 0 0)
          (Utilities|FlowControl|Delay 1.5)
          (Timeline|Timeline Reverse)
          (else
            (Collision|SetCollisionEnabled _staticmesh "QueryOnly")
            (Variables|Default|SetTrapAlreadyActivated false)))))))

(event EventBeginPlay
  ;[0.15 0.15 0.15 0.5] Où est mon static mesh?
  (Variables|Default|SetInitialMeshLocation (Variables|/Script/Engine.SceneComponent|GetRelativeLocation (Variables|Default|GetStaticMesh))))

(fn ConstructionScript)