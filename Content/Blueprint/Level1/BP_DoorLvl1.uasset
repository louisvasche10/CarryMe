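; Double wooden door Blueprint that swings open when the hero punches it.
; OpenDoor, accepted only during the hero's door-punch animation, sets IsLock (actually the "opening" flag) and plays a delayed unlock sound.
; While IsLock is set, Tick interpolates both leaves toward their open angles, setting DoorOpenTrue until both arrive, then clearing IsLock.
; In Scene_Level1 a Gate, opened by the punch animation, guards that rotation; other levels bypass it.
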(event Custom|OpenDoor
  ;[0.15 0.15 0.15 0.5] La porte s'ouvre
  ;;[0.15 0.15 0.15 0.5] Pour eviter que si le joueur spam E la porte s'ouvre quand il passe en AnimationStopPushing
  (if (Variables|/Game/Blueprint/Enemy/BP_Hero.BP_Hero_C|GetAnim_IsPunchingDoor (Variables|Default|GetRefHero))
    (Variables|Default|SetbIsLock true)
    (Utilities|FlowControl|Delay 0.2)
    (Audio|PlaySound2D "/Game/Feedback/SoundEffect/SoundLevel1/SW_Porte_qui_se_déverouille.SW_Porte_qui_se_déverouille" 1.0 1.0 0.0 0 0)))

(event EventTick
  (params (DeltaSeconds :type Float%20%28single-precision%29))
  (bind _sm_door_wood_left (Variables|Components|GetSM_door_wood_left))
  (bind _sm_door_wood_right (Variables|Components|GetSM_door_wood_right))
  ;[0.15 0.15 0.15 0.5] La porte s'ouvre
  (if (== (Variables|Default|GetbIsLock) true)
    ;;[0.15 0.15 0.15 0.5] Le joueur est dans Scene_Level1?
    (bind _returnvalue (Game|GetCurrentLevelName true))
    (if (Utilities|Enum|Equal(Enum) _returnvalue "Scene_Level1")
      (Utilities|FlowControl|Sequence
        (:then_0
          (Utilities|FlowControl|Gate true :!label _label
            (:Exit
              (Transformation|SetRelativeRotation _sm_door_wood_left (Math|Interpolation|RInterpTo (Variables|/Script/Engine.SceneComponent|GetRelativeRotation _sm_door_wood_left) (Math|Rotator|MakeRotator 0.0 0.0 (Variables|Default|GetOpenAngleL)) DeltaSeconds (Variables|Default|GetOpenSeed)) false false :!label _label_2)
              (Transformation|SetRelativeRotation _sm_door_wood_right (Math|Interpolation|RInterpTo (Variables|/Script/Engine.SceneComponent|GetRelativeRotation _sm_door_wood_right) (Math|Rotator|MakeRotator 0.0 0.0 (Variables|Default|GetOpenAngleR)) DeltaSeconds (Variables|Default|GetOpenSeed)) false false)
              (if (and (Math|Float|NearlyEqual(Float) (.Yaw (Math|Rotator|BreakRotator (Variables|/Script/Engine.SceneComponent|GetRelativeRotation _sm_door_wood_left))) (Variables|Default|GetOpenAngleL) 1.0) (Math|Float|NearlyEqual(Float) (.Yaw (Math|Rotator|BreakRotator (Variables|/Script/Engine.SceneComponent|GetRelativeRotation _sm_door_wood_right))) (Variables|Default|GetOpenAngleR) 1.0))
                (Variables|Default|SetbIsLock false)
                (else
                  ;;[0.15 0.15 0.15 0.5] Dire au héro que la porte est ouverte.
                  (Variables|Default|SetDoorOpenTrue? true))))))
        (:then_1
          ;;[0.15 0.15 0.15 0.5] Le joueur ne peux ouvrire la porte temps que le héros n'est pas a un animation.
          (if (Variables|/Game/Blueprint/Enemy/BP_Hero.BP_Hero_C|GetAnim_IsPunchingDoor (Variables|Default|GetRefHero))
            (goto _label Open))))
      (elif (Utilities|Enum|NotEqual(Enum) _returnvalue "Scene_Level1")
        (goto _label_2)))))

(fn ConstructionScript)