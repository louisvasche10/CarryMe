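; Level 1 control panel that lets the player open a linked door, send "debilus" through a hero reference, or trigger a linked trap fall.
; It enables player input at BeginPlay, then unlocks its three input actions after a fixed delay that waits out the dialogue.
; The TriggerGreen overlap shows a hint and sets NearPanel, which the actions never check, and also clears the hero reference.
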(event OnComponentBeginOverlap(TriggerGreen)
  (params (OverlappedComponent :type Primitive%20Component%20Object%20Reference) (OtherActor :type Actor%20Object%20Reference) (OtherComp :type Primitive%20Component%20Object%20Reference) (OtherBodyIndex :type Integer) (bFromSweep :type Boolean) (SweepResult :type Hit%20Result%20Structure%20%28by%20ref%29))
  ;[0.15 0.15 0.15 0.5] le panel que le joueur est là donc le rend accessible
  (Utilities|Casting|CastToBP_FirstPersonCharacter OtherActor)
  (Variables|Default|SetRefHero 0)
  (Variables|Default|SetNearPanel true)
  (Rendering|SetVisibility (Variables|Default|GetHintWidget) true false))

(event Input|EnhancedActionEvents|EnhancedInputActionIA_Interact
  (params (ActionValue :type Boolean) (ElapsedSeconds :type Float%20%28double-precision%29) (TriggeredSeconds :type Float%20%28double-precision%29) (InputAction :type Input%20Action%20Object%20Reference :default "/Game/Input/Actions/IA_Interact.IA_Interact"))
  ;[0.15 0.15 0.15 0.5] la porte s'ouvre quand on appuie sur E
  (if (Variables|Default|GetCanUsePanel)
    (Default|OpenDoor (Variables|Default|GetLinkedDoor))))

(event Input|EnhancedActionEvents|EnhancedInputActionIA_SendDebilus
  (params (ActionValue :type Boolean) (ElapsedSeconds :type Float%20%28double-precision%29) (TriggeredSeconds :type Float%20%28double-precision%29) (InputAction :type Input%20Action%20Object%20Reference :default "/Game/Input/Actions/IA_SendDebilus.IA_SendDebilus"))
  ;[0.15 0.15 0.15 0.5] send debilus quand on appuie sur A
  (if (Variables|Default|GetCanUsePanel)
    (Default|SendDebilus (Variables|Default|GetRefHero))))

(event Input|EnhancedActionEvents|EnhancedInputActionIA_TrapHero
  (params (ActionValue :type Boolean) (ElapsedSeconds :type Float%20%28double-precision%29) (TriggeredSeconds :type Float%20%28double-precision%29) (InputAction :type Input%20Action%20Object%20Reference :default "/Game/Input/Actions/IA_TrapHero.IA_TrapHero"))
  (bind _linkedtrapfall (Variables|Default|GetLinkedTrapFall))
  ;[0.15 0.15 0.15 0.5] le bp_trapfall se déclenche quand on appuie sur W
  (if (Variables|Default|GetCanUsePanel)
    (Utilities|IsValid _linkedtrapfall
      (:Is%20Valid
        (Default|ActivateTrapFall _linkedtrapfall)))))

(event EventBeginPlay
  (Input|EnableInput (Game|GetPlayerController 0))
  ;[0.15 0.15 0.15 0.5] attente de la fin du dialogue avant que le control panel soit utilisable
  (Utilities|FlowControl|Delay 31.0)
  (Variables|Default|SetCanUsePanel true))

(fn ConstructionScript)