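; BP_Boss is a player-controlled pawn for the boss that provides a mouse-driven look camera.
; On BeginPlay it has player controller 0 possess it, adds the IMC_Camera Enhanced Input context, switches to game-only input and hides the cursor.
; IA_Look feeds sensitivity-scaled yaw and inverted pitch, each offset by a stored variable, into controller rotation.
; A comment mentions a bounded view area, but this graph applies no clamp.
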(event Input|EnhancedActionEvents|EnhancedInputActionIA_Look
  (params (ActionValue :type Vector%202D%20Structure) (ElapsedSeconds :type Float%20%28double-precision%29) (TriggeredSeconds :type Float%20%28double-precision%29) (InputAction :type Input%20Action%20Object%20Reference :default "/Game/Blueprint/Boss/IA_Look.IA_Look"))
  (bind (_x _y) (Math|Vector2D|BreakVector2D ActionValue))
  ;[0.15 0.15 0.15 0.5] Regard et zone de vision : la caméra ne peut pas dépasser un certain périmètre
  (Pawn|Input|AddControllerYawInput (+ (* _x (Variables|Default|GetMouseSensitivity)) (Variables|Default|GetCurrentYawn)))
  (Pawn|Input|AddControllerPitchInput (+ (* (* _y -1.0) (Variables|Default|GetMouseSensitivity)) (Variables|Default|GetCurrentPitch))))

(event EventBeginPlay
  (bind _returnvalue (Game|GetPlayerController 0))
  ;[0.15 0.15 0.15 0.5] 📞Oui allo? je voudrais un IMC_Camera, merci
  (Input|EnableInput _returnvalue)
  (Pawn|Possess _returnvalue self)
  (Input|AddMappingContext (PlayerController|LocalPlayerSubsystems|GetEnhancedInputLocalPlayerSubsystem _returnvalue) "/Game/Blueprint/Boss/IMC_Camera.IMC_Camera" 0 "(bIgnoreAllPressedKeysUntilRelease=True,bForceImmediately=False,bNotifyUserSettings=False)")
  (Input|SetInputModeGameOnly _returnvalue false)
  (Variables|/Script/Engine.PlayerController|SetbShowMouseCursor _returnvalue false))

(fn ConstructionScript)