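; BP_DialogueHidden is a dialogue trigger actor that shows its Dialogue through the first-person player controller when the hero enters its box.
; BeginPlay disables the box's collision and caches the player controller, so the trigger stays dormant unless collision is enabled from outside this graph.
; The overlap handler accepts only BP_Hero and uses DoOnce to fire the dialogue a single time.
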(event OnComponentBeginOverlap(Box)
  (params (OverlappedComponent :type Primitive%20Component%20Object%20Reference) (OtherActor :type Actor%20Object%20Reference) (OtherComp :type Primitive%20Component%20Object%20Reference) (OtherBodyIndex :type Integer) (bFromSweep :type Boolean) (SweepResult :type Hit%20Result%20Structure%20%28by%20ref%29))
  (bind _asbp_hero (Utilities|Casting|CastToBP_Hero OtherActor))
  (Utilities|FlowControl|DoOnce false
    (:Completed
      (Default|ShowDialogue (Variables|Default|Getplayercontroller) (Variables|Default|GetDialogue)))))

(event EventBeginPlay
  (Collision|SetCollisionEnabled (Variables|Default|GetBox) "NoCollision")
  (bind _asbp_first_person_player_controller (Utilities|Casting|CastToBP_FirstPersonPlayerController (Game|GetPlayerController 0)))
  (Variables|Default|Setplayercontroller _asbp_first_person_player_controller))

(fn ConstructionScript)