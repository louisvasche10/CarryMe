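; BP_DialogueTriggerHero is a trigger volume that shows a dialogue when the hero enters its box.
; BeginPlay caches the first-person player controller.
; The first overlap passes a DoOnce, then casts the actor to BP_Hero, optionally waits a few seconds for the level 1 door dialogue, and calls ShowDialogue on the controller.
; Because the DoOnce precedes the cast, any earlier non-hero overlap uses up the trigger.
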(event OnComponentBeginOverlap(Box)
  (params (OverlappedComponent :type Primitive%20Component%20Object%20Reference) (OtherActor :type Actor%20Object%20Reference) (OtherComp :type Primitive%20Component%20Object%20Reference) (OtherBodyIndex :type Integer) (bFromSweep :type Boolean) (SweepResult :type Hit%20Result%20Structure%20%28by%20ref%29))
  (Utilities|FlowControl|DoOnce false
    (:Completed
      (Development|PrintString "OVERLAP BOX")
      (bind _asbp_hero (Utilities|Casting|CastToBP_Hero OtherActor))
      ;[0.15 0.15 0.15 0.5] Permet que dans le level 1 le dialogues de la porte est un delai avant de s'activer
      (if (Variables|Default|GetHasDelay)
        (Utilities|FlowControl|Delay 4.0))
      (Default|ShowDialogue (Variables|Default|Getplayercontroller) (Variables|Default|GetDialogue)))))

(event EventBeginPlay
  (bind _asbp_first_person_player_controller (Utilities|Casting|CastToBP_FirstPersonPlayerController (Game|GetPlayerController 0)))
  (Variables|Default|Setplayercontroller _asbp_first_person_player_controller))

(fn ConstructionScript)