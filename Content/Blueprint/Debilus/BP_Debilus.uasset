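; BP_Debilus is a skeletal-mesh actor that can walk and be knocked into a ragdoll.
; SetDebilusWalking passes the walking flag to the ABP_Debilus3 animation Blueprint.
; StartDebilusRadgoll switches the mesh to ragdoll physics, launches it with a fixed velocity-change impulse after a brief delay, then destroys the actor two seconds later.
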(event Custom|StartDebilusRadgoll
  (bind _mesh (Variables|Character|GetMesh))
  (Variables|Default|SetbIsRagdoll true)
  (Collision|SetCollisionProfileName _mesh "Ragdoll" true :!class /Script/Engine.PrimitiveComponent)
  (Collision|SetCollisionEnabled _mesh "QueryAndPhysics")
  (Class|SkeletalMeshComponent|SetAllBodiesSimulatePhysics _mesh true)
  (Class|PrimitiveComponent|WakeAllRigidBodies _mesh)
  (Utilities|FlowControl|Delay 0.05)
  (Physics|AddImpulse _mesh "0.000000,2000.000000,3000.000000" "None" true)
  (Utilities|FlowControl|Delay 2.0)
  (Actor|DestroyActor))

(event Custom|SetDebilusWalking
  (params (Walking :type Boolean))
  (bind _asabp_debilus_3 (Utilities|Casting|CastToABP_Debilus3 (Components|SkeletalMesh|GetAnimInstance (Variables|Character|GetMesh))))
  (Variables|/Game/Characters/Debilus3/Debilus3_Skeleton/ABP_Debilus3.ABP_Debilus3_C|SetIsWalking _asabp_debilus_3 Walking))

(fn ConstructionScript)