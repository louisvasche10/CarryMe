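; Scripted hero character that plays staged sequences across several levels: walking, inspecting, pushing doors, reacting to traps and punching Debilus.
; A HeroState machine in TransitionTo sets anim flags, speed and active spline, while Tick moves the hero along that spline and spline ends or delay events chain the next state.
; Trap hits ragdoll the hero and respawn it, timelines drive the widget-triggered Debilus scene and slow motion, and polling waits on doors.
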(event Custom|OnSplineEnd
  ;[0.15 0.15 0.15 0.5] A la fin d'un spline permet au héros de chosir un nouveau spline et de le suivre.
  (Variables|Default|SetbIsMoving false)
  (Utilities|FlowControl|Sequence
    (:then_0
      (if (Utilities|Enum|Equal(Enum) (Variables|Default|GetHeroState) "NewEnumerator0")
        (switch Utilities|FlowControl|Switch|SwitchonE_HeroState (Variables|Default|GetHeroState)
          (:NewEnumerator0
            (CallFunction|Transitionto "NewEnumerator3")))))
    (:then_1
      (if (Utilities|Enum|Equal(Enum) (Variables|Default|GetHeroState) "NewEnumerator24")
        (CallFunction|Transitionto "NewEnumerator18")))
    (:then_2
      (if (Utilities|Enum|Equal(Enum) (Variables|Default|GetHeroState) "NewEnumerator25")
        (CallFunction|Transitionto "NewEnumerator28")
        (else
          (bind _returnvalue (Actor|GetActorOfClass "/Game/Blueprint/level2/BP_DoorLvl2.BP_DoorLvl2_C"))
          (if (and (Utilities|Enum|Equal(Enum) (Variables|Default|GetHeroState) "NewEnumerator30") (Variables|/Game/Blueprint/level2/BP_DoorLvl2.BP_DoorLvl2_C|GetbIsLock _returnvalue))
            (CallFunction|Transitionto "NewEnumerator31")))))))

(event Custom|DoeasyWalkDelay
  ;[0.15 0.15 0.15 0.5] Dans la fonction Transition To on a besoin de delay des fois, les voila
  ;;[0.15 0.15 0.15 0.5] Level 2
  (Utilities|FlowControl|DoN 1
    (:Exit
      (Utilities|FlowControl|Delay 6.0)
      (CallFunction|Transitionto "NewEnumerator13"))))

(event Custom|DelayAfterGetUp
  ;[0.15 0.15 0.15 0.5] Dans la fonction Transition To on a besoin de delay des fois, les voila
  ;;[0.15 0.15 0.15 0.5] LVL 1
  ;;;[0.15 0.15 0.15 0.5] Aprer avoir pousser la porte
  (Utilities|FlowControl|Delay 8.5)
  (CallFunction|Transitionto "NewEnumerator22"))

(event Custom|OnTrapHit
  ;[0.15 0.15 0.15 0.5] Lance le ragdoll quand le hero se prend le piège, A SIMPLIFIER
  (Utilities|FlowControl|Delay 1.0)
  (if (Utilities|Enum|Equal(Enum) (Variables|Default|GetHeroState) "NewEnumerator3")
    (CallFunction|StartTrapRagdoll1)
    (elif (Utilities|Enum|Equal(Enum) (Variables|Default|GetHeroState) "NewEnumerator6")
      (CallFunction|ResetAnim)
      (CallFunction|StartTrapRagdoll2))))

(event Custom|DelayAfterFalling
  ;[0.15 0.15 0.15 0.5] Dans la fonction Transition To on a besoin de delay des fois, les voila
  ;;[0.15 0.15 0.15 0.5] LVL 1
  ;;;[0.15 0.15 0.15 0.5] Aprer avoir pousser la porte
  (Utilities|FlowControl|Delay 0.7)
  (Audio|PlaySound2D "/Game/Feedback/SoundEffect/SoundLevel1/SW_HeroFallGround.SW_HeroFallGround" 1.0 1.0 0.0 0 0)
  (Utilities|FlowControl|Delay 3.0)
  (Variables|AnimLvl1|SetAnimIsDoorHeroFalling false)
  (Variables|Default|SetbIsMoving true)
  (Variables|Default|SetDistanceAlongSpline 0.0)
  (Utilities|FlowControl|Delay 0.0)
  (CallFunction|Transitionto "NewEnumerator20"))

(event Custom|DelayBeforWalkAfterLookingButWhileWhenLookingInTheLevelOne
  ;[0.15 0.15 0.15 0.5] Dans la fonction Transition To on a besoin de delay des fois, les voila
  ;;[0.15 0.15 0.15 0.5] LVL 1
  (Utilities|FlowControl|Delay 2.0)
  (CallFunction|Transitionto "NewEnumerator23"))

(event Custom|Roll
  (Variables|AnimLvl1|SetAnimIsRoll true)
  (Variables|Default|SetWalkSpeed 3e+02)
  (Utilities|FlowControl|Delay 1.0)
  (Variables|AnimLvl1|SetAnimIsRoll false)
  (Variables|AnimForAll|SetAnim_IsWalking false)
  (Variables|AnimForAll|SetAnim_IsSneak true)
  (Variables|Default|SetWalkSpeed 2e+02)
  (Utilities|FlowControl|Delay 4.0)
  (Variables|Default|SetWalkSpeed 3e+02)
  (Variables|AnimForAll|SetAnim_IsSneak false)
  (Variables|AnimLvl1|SetAnimIsRoll true)
  (Utilities|FlowControl|Delay 1.0)
  (Variables|AnimLvl1|SetAnimIsRoll false)
  (Variables|AnimForAll|SetAnim_IsSneak true)
  (Variables|Default|SetWalkSpeed 2e+02))

(event Custom|StartTrapRagdoll1
  ;[0.15 0.15 0.15 0.5] Lance le ragdoll quand le hero se prend le piège, A SIMPLIFIER
  (Variables|Default|SetHeroState "NewEnumerator5")
  (CallFunction|StartHeroRagdoll)
  (Utilities|FlowControl|Delay 4.0)
  (CallFunction|StopHeroRagdoll))

(event Custom|DelayJump
  ;[0.15 0.15 0.15 0.5] Dans la fonction Transition To on a besoin de delay des fois, les voila
  ;;[0.15 0.15 0.15 0.5] lvl3
  (Variables|Anim_Lvl3|SetAnim_IsJumping true))

(event Custom|SlowerTimeline
  (bind _alpha (Timeline|Slow PlayFromStart)
    (:Update
      (Utilities|Time|SetGlobalTimeDilation _alpha))
    (:Finished
      (bind _alpha_2 (Timeline|Fast PlayFromStart)
        (:Update
          (Utilities|Time|SetGlobalTimeDilation _alpha_2))))))

(event Custom|SendDebilus
  ;[0.15 0.15 0.15 0.5] Après validation du widget, on appuis sur E via le custom event SendDebilus. Debilus apparaît derrière le héros.
  ; Une Timeline le déplace vers un TargetPoint placé dans la scène.
  ; Quand Debilus arrive, le héros se rapproche de lui le tape, puis Debilus passe en ragdoll avant de disparaître.
  ; La séquence se termine en lançant GuardStance.
  (if (Utilities|Enum|Equal(Enum) (Variables|Default|GetHeroState) "NewEnumerator9")
    (bind _foundwidgets (Widget|GetAllWidgetsOfClass "/Game/Widget/WBP_SendDebilus.WBP_SendDebilus_C" true))
    (Widget|RemovefromParent (Utilities|Array|Get(acopy) _foundwidgets))
    (CallFunction|Transitionto "NewEnumerator10")))

(event Custom|StartHeroMoveToDebilus
  ;[0.15 0.15 0.15 0.5] Après validation du widget, on appuis sur E via le custom event SendDebilus. Debilus apparaît derrière le héros.
  ; Une Timeline le déplace vers un TargetPoint placé dans la scène.
  ; Quand Debilus arrive, le héros se rapproche de lui le tape, puis Debilus passe en ragdoll avant de disparaître.
  ; La séquence se termine en lançant GuardStance.
  (Default|SetDebilusWalking (Variables|Default|GetDebilusRef) false)
  (Variables|Default|SetHeroStartLocation (Transformation|GetActorLocation))
  (Variables|Default|SetHeroAttackLocation (+ (Transformation|GetActorLocation (Variables|Default|GetDebilusRef)) (* (Math|Vector|Normalize (- (Transformation|GetActorLocation) (Transformation|GetActorLocation (Variables|Default|GetDebilusRef)))) (Variables|Default|GetFloat2))))
  (bind _alpha (Timeline|TL_HeroMoveToDebilus PlayFromStart)
    (:Update
      (if (Variables|Default|GetPunchDébilusAgain?)
        (Variables|AnimLvl2|SetAnim_IsAngryRunning true)
        (Transformation|SetActorLocation (Math|Vector|Lerp(Vector) (Variables|Default|GetHeroStartLocation) (Variables|Default|GetHeroAttackLocation) _alpha) false false)
        (Utilities|FlowControl|Delay 1.5)
        (Variables|AnimLvl2|SetAnim_IsAngryRunning false)
        (Variables|AnimLvl2|SetAnim_IsPunching true)
        (Utilities|FlowControl|Delay 1.0)
        (CallFunction|HitDebilus)
        (else
          ;;[0.15 0.15 0.15 0.5] EMPCHE LE SONS DE FRAPPER DéBILUS SE JOUE 2 FOIX
          (Development|PrintString "FAUX" true true "(R=0.000000,G=1.000000,B=0.302052,A=1.000000)" 2e+01))))))

(event Custom|AfterLook
  ;[0.15 0.15 0.15 0.5] Dans la fonction Transition To on a besoin de delay des fois, les voila
  ;;[0.15 0.15 0.15 0.5] LVL 1
  ;;;[0.15 0.15 0.15 0.5] Début / regarder / marcher / pousser
  (Utilities|FlowControl|Delay 3.0)
  (CallFunction|Transitionto "NewEnumerator24"))

(event Custom|HitDebilus
  ;[0.15 0.15 0.15 0.5] Après validation du widget, on appuis sur E via le custom event SendDebilus. Debilus apparaît derrière le héros.
  ; Une Timeline le déplace vers un TargetPoint placé dans la scène.
  ; Quand Debilus arrive, le héros se rapproche de lui le tape, puis Debilus passe en ragdoll avant de disparaître.
  ; La séquence se termine en lançant GuardStance.
  ;;[0.15 0.15 0.15 0.5] 👊Dans ta gueule Débilus
  (Utilities|FlowControl|DoN 1
    (:Exit
      (Audio|PlaySound2D "/Game/Feedback/SoundEffect/SoundLevel2/SW_HeroPunchDebilus.SW_HeroPunchDebilus" 1.0 1.0 0.0 0 0)
      (bind _debilusref (Variables|Default|GetDebilusRef)
        (:then
          (Default|StartDebilusRadgoll _debilusref)
          (Utilities|FlowControl|Delay 4.0)
          (CallFunction|Transitionto "NewEnumerator12"))
        (:else)))))

(event Custom|StartInspectPause
  ;[0.15 0.15 0.15 0.5] Déplace le heros sur la spline actuelle stockée dasn activeSpline.
  ;;[0.15 0.15 0.15 0.5] Cette partie sert a ce que quand il se balade la premiere fois, il puisse s'arreter a different endroit pour faire des animation d'inspection puis reprendre sa marche
  ;;;[0.15 0.15 0.15 0.5] Temps d'inspection
  (Variables|Default|SetbIsMoving false)
  (Variables|AnimForAll|SetAnim_IsWalking false)
  (Variables|AnimLvl2|SetAnim_IsLookingAround true)
  (Utilities|FlowControl|Delay 3.0)
  (Variables|AnimLvl2|SetAnim_IsLookingAround false)
  (Variables|Default|SetbIsMoving true)
  (Variables|AnimForAll|SetAnim_IsWalking true))

(event Custom|BackTimeline
  (bind _alpha (Timeline|Slow Stop)
    (:Update
      (Utilities|Time|SetGlobalTimeDilation _alpha))
    (:Finished
      (bind _alpha_2 (Timeline|Fast PlayFromStart)
        (:Update
          (Utilities|Time|SetGlobalTimeDilation _alpha_2))))))

(event Custom|DelayDance
  ;[0.15 0.15 0.15 0.5] Dans la fonction Transition To on a besoin de delay des fois, les voila
  ;;[0.15 0.15 0.15 0.5] Level 2
  ;;;[0.15 0.15 0.15 0.5] Combien de temps il danse
  (Utilities|FlowControl|Delay 4.0))

(event Custom|DelayDeconnard
  (Utilities|FlowControl|Delay 6.0))

(event Custom|DelayForGetUp
  (Utilities|FlowControl|Delay 7.0)
  (CallFunction|Transitionto "NewEnumerator30")
  (Audio|PlaySound2D "/Game/Feedback/SoundEffect/RéapparitionHero.RéapparitionHero" 1.0 1.0 0.0 0 0)
  (Actor|Tick|SetActorTickEnabled true)
  (Variables|AnimLvl1|SetAnimIsGetUp false))

(event Custom|ItsGood?DoorIsOpen?
  (Utilities|Time|SetTimerbyEvent (delegate Custom|CustomEvent) 0.5 true))

(event Custom|CustomEvent
  (bind _returnvalue (Actor|GetActorOfClass "/Game/Blueprint/level2/BP_DoorLvl2.BP_DoorLvl2_C"))
  (if (not (Variables|/Game/Blueprint/level2/BP_DoorLvl2.BP_DoorLvl2_C|GetbIsLock _returnvalue))
    (Variables|AnimLvl2|SetAnim_WtfDoorIsNotOpen false)
    (Utilities|FlowControl|DoN 1
      (:Exit
        (CallFunction|Transitionto "NewEnumerator32")))))

(event Custom|ShowDebilusWidget
  ;[0.15 0.15 0.15 0.5] Après validation du widget, on appuis sur E via le custom event SendDebilus. Debilus apparaît derrière le héros.
  ; Une Timeline le déplace vers un TargetPoint placé dans la scène.
  ; Quand Debilus arrive, le héros se rapproche de lui le tape, puis Debilus passe en ragdoll avant de disparaître.
  ; La séquence se termine en lançant GuardStance.
  (bind _returnvalue (UserInterface|CreateWidget "/Game/Widget/WBP_SendDebilus.WBP_SendDebilus_C"))
  (UserInterface|Viewport|AddtoViewport _returnvalue 0)
  (Widget|SetKeyboardFocus _returnvalue))

(event Custom|StartDebilusSequence
  (bind _debilusdestinationref (Variables|Default|GetDebilusDestinationRef))
  (bind _debilusref (Variables|Default|GetDebilusRef))
  (bind _returnvalue (Transformation|GetActorLocation _debilusdestinationref))
  (bind _mesh (Variables|/Script/Engine.Character|GetMesh _debilusref))
  (bind (_x _y) (Math|Vector|BreakVector _returnvalue))
  ;[0.15 0.15 0.15 0.5] Après validation du widget, on appuis sur E via le custom event SendDebilus. Debilus apparaît derrière le héros.
  ; Une Timeline le déplace vers un TargetPoint placé dans la scène.
  ; Quand Debilus arrive, le héros se rapproche de lui le tape, puis Debilus passe en ragdoll avant de disparaître.
  ; La séquence se termine en lançant GuardStance.
  (bind _debilusref_2 (Variables|Default|GetDebilusRef)
    (:then
      (Variables|Default|SetbIsMoving false)
      (Physics|SetSimulatePhysics (Variables|/Script/Engine.Character|GetMesh _debilusref_2) false)
      (Collision|SetCollisionEnabled (Variables|/Script/Engine.Character|GetMesh _debilusref_2) "NoCollision")
      (Transformation|SetRelativeLocation (Variables|/Script/Engine.Character|GetMesh _debilusref_2) "0.000000,0.000000,-90.000000" false false)
      (Transformation|SetRelativeRotation (Variables|/Script/Engine.Character|GetMesh _debilusref_2) "0.000000,-70.000000,0.000000" false false)
      (Transformation|SetActorLocation _debilusref_2 (- (Transformation|GetActorLocation) (* (Transformation|GetActorForwardVector) (Variables|Default|GetFloat))) false true)
      (Rendering|SetActorHiddenInGame _debilusref false)
      (Default|SetDebilusWalking _debilusref true)
      (Physics|SetSimulatePhysics _mesh false)
      (Collision|SetCollisionEnabled _mesh "NoCollision")
      (Variables|Default|SetDebilusStartLocation "540.000000,-930.000000,-312.000000")
      (Variables|Default|SetDebilusEndLocation (Math|Vector|MakeVector _x _y -312.0))
      (bind _alpha (Timeline|TL_DebilusWalk PlayFromStart)
        (:Update
          (Transformation|SetActorLocation (Variables|Default|GetDebilusRef) (Math|Vector|Lerp(Vector) (Variables|Default|GetDebilusStartLocation) (Variables|Default|GetDebilusEndLocation) _alpha) false false))
        (:Finished
          (Default|SetDebilusWalking (Variables|Default|GetDebilusRef) false)
          (CallFunction|StartHeroMovetoDebilus))))
    (:else)))

(event Custom|DoorIsOpen?
  ;[0.15 0.15 0.15 0.5] Dans la fonction Transition To on a besoin de delay des fois, les voila
  ;;[0.15 0.15 0.15 0.5] LVL 1
  ;;;[0.15 0.15 0.15 0.5] Début / regarder / marcher / pousser
  (if (Variables|/Game/Blueprint/Level1/BP_DoorLvl1.BP_DoorLvl1_C|GetDoorOpenTrue? (Variables|Default|GetRefDoor))
    (Variables|AnimLvl1|SetAnim_IsPunchingDoor false)
    (CallFunction|Transitionto "NewEnumerator19")
    (else
      (Utilities|FlowControl|Delay 0.2)
      (CallFunction|DoorIsOpen?))))

(event Custom|DoAngryDelay
  ;[0.15 0.15 0.15 0.5] Dans la fonction Transition To on a besoin de delay des fois, les voila
  ;;[0.15 0.15 0.15 0.5] Level 2
  (Utilities|FlowControl|Delay 4.0)
  (Variables|AnimLvl2|SetAnim_IsStunned false)
  (CallFunction|Transitionto "NewEnumerator6"))

(event Custom|AfterWalkPushDoor
  ;[0.15 0.15 0.15 0.5] Dans la fonction Transition To on a besoin de delay des fois, les voila
  ;;[0.15 0.15 0.15 0.5] LVL 1
  ;;;[0.15 0.15 0.15 0.5] Début / regarder / marcher / pousser
  (CallFunction|Transitionto "NewEnumerator18"))

(event Custom|DoThinkingDelay
  ;[0.15 0.15 0.15 0.5] Dans la fonction Transition To on a besoin de delay des fois, les voila
  ;;[0.15 0.15 0.15 0.5] Level 2
  (CallFunction|Transitionto "NewEnumerator9"))

(event Custom|StartTrapRagdoll2
  ;[0.15 0.15 0.15 0.5] Lance le ragdoll quand le hero se prend le piège, A SIMPLIFIER
  (Variables|Default|SetHeroState "NewEnumerator8")
  (CallFunction|StartHeroRagdoll)
  (Utilities|FlowControl|Delay 6.0)
  (CallFunction|StopHeroRagdoll))

(event EventBeginPlay
  ;[0.15 0.15 0.15 0.5] Au lancement, on enregistre seulement la position de spawn puis on lance l’état StartState via le detail du hero sur la scène.
  ; Toutes les valeurs de vitesse, spline active et mouvement doivent être configurées dans TransitionTo pour éviter les conflits.
  (Input|EnableInput self (Game|GetPlayerController 0))
  (Variables|Default|SetSpawnLocation (Transformation|GetActorLocation))
  (Variables|Default|SetHeroState (Variables|Default|GetStartState))
  (if (Utilities|Enum|Equal(Enum) (Variables|Default|GetHeroState) "NewEnumerator0")
    (Variables|Default|SetDistanceAlongSpline 0.0)
    (Variables|spline|SetActiveSplineRef (Variables|SplineLvl2|GetExplorationSplineRef))
    (Variables|Default|SetbIsMoving true)
    (Variables|AnimForAll|SetAnim_IsSneak true)
    (Actor|Tick|SetActorTickEnabled true)
    (elif (Utilities|Enum|Equal(Enum) (Variables|Default|GetHeroState) "NewEnumerator15")
      (CallFunction|Transitionto "NewEnumerator15")
      (Variables|spline|SetActiveSplineRef (Variables|SplineLvl1|Getdeplacementniv1))
      (Variables|Default|SetbIsMoving true)
      (Actor|Tick|SetActorTickEnabled true))))

(event EventTick
  (params (DeltaSeconds :type Float%20%28single-precision%29))
  ;[0.15 0.15 0.15 0.5] Déplace le heros sur la spline actuelle stockée dasn activeSpline.
  (if (Variables|Default|GetbIsMoving)
    (Variables|Default|SetDistanceAlongSpline (+ (* (Variables|Default|GetWalkSpeed) DeltaSeconds) (Variables|Default|GetDistanceAlongSpline)))
    (if (>= (Variables|Default|GetDistanceAlongSpline) (Spline|GetSplineLength (Variables|/Game/Blueprint/Enemy/BP_SplinePath.BP_SplinePath_C|GetSpline (Variables|spline|GetActiveSplineRef))))
      (CallFunction|OnSplineEnd)
      (else
        (Transformation|SetActorLocation (Spline|GetLocationatDistanceAlongSpline (Variables|/Game/Blueprint/Enemy/BP_SplinePath.BP_SplinePath_C|GetSpline (Variables|spline|GetActiveSplineRef)) (Variables|Default|GetDistanceAlongSpline) "World") false false)
        (Transformation|SetActorRotation (Math|Rotator|CombineRotators (Math|Conversions|RotationFromXVector (Spline|GetDirectionatDistanceAlongSpline (Variables|/Game/Blueprint/Enemy/BP_SplinePath.BP_SplinePath_C|GetSpline (Variables|spline|GetActiveSplineRef)) (Variables|Default|GetDistanceAlongSpline) "World")) (Math|Rotator|MakeRotator 0.0 0.0 0.0)))
        ;;[0.15 0.15 0.15 0.5] Cette partie sert a ce que quand il se balade la premiere fois, il puisse s'arreter a different endroit pour faire des animation d'inspection puis reprendre sa marche
        ;;;[0.15 0.15 0.15 0.5] Roulade sexy
        (if (and (Utilities|Enum|Equal(Enum) (Variables|Default|GetHeroState) "NewEnumerator24") (>= (Variables|Default|GetDistanceAlongSpline) (Variables|Default|GetRollPoint)))
          (CallFunction|Roll)
          (elif (and (Utilities|Enum|Equal(Enum) (Variables|Default|GetHeroState) "NewEnumerator25") (>= (Variables|Default|GetDistanceAlongSpline) (Variables|Default|GetLookPoint)))
            (Utilities|FlowControl|DoN 1
              (:Exit
                (CallFunction|StartInspectPause)))))))))

(fn ConstructionScript)

(fn Transitionto
  (params (NewState :type E_HeroState%20Enum :default "NewEnumerator0"))
  (bind _refsplinelvl1look (Variables|SplineLvl1|GetRefSplineLvl1Look))
  ;[0.15 0.15 0.15 0.5] Toute les transition dans lequel le heros va passer dans le level 2
  (bind _output_get (Variables|Default|SetHeroState NewState))
  (Development|PrintString (Utilities|String|EnumtoString _output_get))
  (CallFunction|ResetAnim)
  (switch Utilities|FlowControl|Switch|SwitchonE_HeroState NewState
    (:NewEnumerator0
      (Variables|Default|SetDistanceAlongSpline 0.0)
      (Variables|spline|SetActiveSplineRef (Variables|SplineLvl2|GetExplorationSplineRef))
      (Variables|Default|SetbIsMoving true)
      (Variables|AnimForAll|SetAnim_IsSneak true))
    (:NewEnumerator3
      (Variables|AnimForAll|SetAnim_IsSneak false)
      (Variables|Default|SetWalkSpeed 4e+01)
      (Variables|Default|SetDistanceAlongSpline 0.0)
      (Variables|spline|SetActiveSplineRef (Variables|SplineLvl2|GetApproachSplineRef))
      (Variables|Default|SetbIsMoving true)
      (Variables|AnimLvl2|SetAnim_IsTipToeing true))
    (:NewEnumerator5
      (Variables|Default|SetbIsMoving false)
      (Variables|AnimLvl2|SetAnim_IsStunned true)
      (CallFunction|DoAngryDelay))
    (:NewEnumerator6
      (Variables|Default|SetWalkSpeed 5e+02)
      (Variables|Default|SetDistanceAlongSpline 0.0)
      (Variables|spline|SetActiveSplineRef (Variables|SplineLvl2|GetAngrySplineRef))
      (Variables|Default|SetbIsMoving true)
      (Variables|AnimLvl2|SetAnim_IsTipToeing false)
      (Variables|AnimLvl2|SetAnim_IsAngryRunning true))
    (:NewEnumerator8
      (Variables|Default|SetbIsMoving false)
      (Variables|AnimLvl2|SetAnim_ISThinking true)
      (CallFunction|DoThinkingDelay))
    (:NewEnumerator9
      (Variables|Default|SetbIsMoving false)
      (Variables|AnimLvl2|SetAnim_ISThinking true)
      (CallFunction|ShowDebilusWidget))
    (:NewEnumerator10
      (Variables|Default|SetbIsMoving false)
      (Variables|AnimLvl2|SetAnim_ISThinking false)
      (CallFunction|StartDebilusSequence))
    (:NewEnumerator12
      (Variables|Default|SetWalkSpeed 4.5e+02)
      (Variables|Default|SetDistanceAlongSpline 0.0)
      (Variables|spline|SetActiveSplineRef (Variables|SplineLvl2|GetEasySplineRef))
      (Variables|Default|SetbIsMoving true)
      (Variables|AnimLvl2|SetAnim_IsAngryRunning true)
      (CallFunction|DoeasyWalkDelay))
    (:NewEnumerator13
      (Variables|Default|SetbIsMoving false)
      (Variables|AnimLvl2|SetAnim_IsAngryRunning false)
      (Variables|AnimLvl2|SetAnim_IsVictoryDancing true)
      (CallFunction|DelayDance))
    (:NewEnumerator30
      (Variables|spline|SetActiveSplineRef (Variables|SplineLvl2|GetSplineFinaleLvl2))
      (Variables|Default|SetDistanceAlongSpline 0.0)
      (Variables|Default|SetbIsMoving true)
      (Variables|AnimForAll|SetAnim_IsWalking true)
      (Variables|Default|SetWalkSpeed 2.5e+02))
    (:NewEnumerator31
      (Variables|Default|SetbIsMoving false)
      (Variables|AnimLvl1|SetAnimIsGetUp false)
      (Variables|AnimLvl2|SetAnim_WtfDoorIsNotOpen true)
      (CallFunction|ItsGood?DoorIsOpen?))
    (:NewEnumerator32
      (Variables|spline|SetActiveSplineRef (Variables|SplineLvl2|GetSplineRealyFinalWalk))
      (Variables|Default|SetDistanceAlongSpline 0.0)
      (Variables|Default|SetbIsMoving true)
      (Variables|AnimForAll|SetAnim_IsWalking true)
      (Variables|Default|SetWalkSpeed 2.5e+02))
    (:NewEnumerator15
      ;[0.15 0.15 0.15 0.5] LEVEL 1 / marche -> pousse porte -> abbandonne -> marche
      (Variables|Default|SetDistanceAlongSpline 0.0)
      (Variables|spline|SetActiveSplineRef (Variables|SplineLvl1|Getdeplacementniv1))
      (Variables|Default|SetbIsMoving true)
      (Variables|AnimForAll|SetAnim_IsWalking true)
      (CallFunction|DelayBeforWalkAfterLookingButWhilewhenLookingintheLevelOne))
    (:NewEnumerator23
      (Variables|Default|SetbIsMoving false)
      (Variables|AnimLvl1|SetAnimeIsLvl1Look true)
      (CallFunction|AfterLook))
    (:NewEnumerator24
      (Variables|AnimLvl1|SetAnimeIsLvl1Look false)
      (Variables|Default|SetDistanceAlongSpline 0.0)
      (Variables|AnimForAll|SetAnim_IsWalking true)
      (Variables|spline|SetActiveSplineRef _refsplinelvl1look)
      (Development|PrintString (Utilities|GetDisplayName _refsplinelvl1look))
      (Variables|Default|SetbIsMoving true))
    (:NewEnumerator18
      (Variables|Default|SetbIsMoving false)
      (Variables|AnimLvl1|SetAnim_IsPunchingDoor true)
      (Variables|AnimForAll|SetAnim_IsWalking false)
      (CallFunction|DoorIsOpen?))
    (:NewEnumerator19
      (Variables|spline|SetActiveSplineRef (Variables|SplineLvl1|GetWalkIfDoorOpen))
      (Variables|AnimLvl1|SetAnimIsDoorHeroFalling true)
      (CallFunction|DelayAfterFalling))
    (:NewEnumerator20
      (Variables|AnimLvl1|SetAnimIsGetUp true)
      (Variables|Default|SetbIsMoving false)
      (CallFunction|DelayAfterGetUp))
    (:NewEnumerator22
      (Variables|Default|SetbIsMoving true)
      (Variables|AnimForAll|SetAnim_IsSneak true))
    (:NewEnumerator25
      ;[0.15 0.15 0.15 0.5] Level 3?
      (Variables|Default|SetDistanceAlongSpline 0.0)
      (Variables|spline|SetActiveSplineRef (Variables|Spline_Lvl3|GetSplineLvl3))
      (Variables|Default|SetbIsMoving true)
      (Variables|AnimForAll|SetAnim_IsWalking true)
      (Variables|Default|SetWalkSpeed 3e+02)
      (Actor|Tick|SetActorTickEnabled true))
    (:NewEnumerator26
      (Variables|Default|SetDistanceAlongSpline 0.0)
      (Variables|spline|SetActiveSplineRef (Variables|Spline_Lvl3|GetSpline_Run&Jump))
      (Variables|Default|SetbIsMoving true)
      (Variables|AnimForAll|SetAnim_IsWalking false)
      (Variables|AnimLvl2|SetAnim_IsAngryRunning true)
      (Variables|Default|SetWalkSpeed 5e+02))
    (:NewEnumerator28
      (CallFunction|DelayJump)
      (Actor|Tick|SetActorTickEnabled true))))

(fn ResetAnim
  (Variables|AnimLvl2|SetAnim_IsTipToeing false)
  (Variables|AnimLvl2|SetAnim_IsStunned false)
  (Variables|AnimLvl2|SetAnim_IsLookingAround false)
  (Variables|AnimLvl2|SetAnim_ISThinking false)
  (Variables|AnimLvl2|SetAnim_IsPunching false)
  (Variables|AnimLvl2|SetAnim_IsAngryRunning false)
  (Variables|AnimLvl2|SetAnim_IsVictoryDancing false)
  (Variables|Anim_Lvl3|SetAnim_IsJumping false)
  (Variables|AnimForAll|SetAnim_IsWalking false))

(fn StartHeroRagdoll
  (bind _mesh (Variables|Character|GetMesh))
  (Variables|Default|SetbIsRagdoll true)
  (Variables|Default|SetbIsMoving false)
  (Variables|AnimForAll|SetAnim_IsWalking false)
  (CallFunction|ResetAnim)
  (Collision|SetCollisionEnabled (Variables|Collision|GetCapsuleComponent) "NoCollision")
  (Collision|SetCollisionProfileName _mesh "Ragdoll" true :!class /Script/Engine.PrimitiveComponent)
  (Collision|SetCollisionEnabled _mesh "QueryAndPhysics")
  (Physics|SetSimulatePhysics _mesh true)
  (Class|PrimitiveComponent|WakeAllRigidBodies _mesh)
  (Physics|AddImpulse _mesh "750.000000,0.000000,4000.000000" "" true))

(fn StopHeroRagdoll
  (bind _mesh (Variables|Character|GetMesh))
  (bind _capsulecomponent (Variables|Collision|GetCapsuleComponent))
  (bind _mesh_2 (Variables|Character|GetMesh))
  (Physics|SetSimulatePhysics _mesh false)
  (Collision|SetCollisionEnabled _mesh "NoCollision")
  (Collision|SetCollisionEnabled _capsulecomponent "QueryAndPhysics")
  (Collision|SetCollisionProfileName _capsulecomponent "Pawn" true :!class /Script/Engine.PrimitiveComponent)
  (Transformation|SetActorLocation (Variables|Default|GetSpawnLocation) false true)
  (Transformation|SetRelativeLocation _mesh_2 "0.000000,0.000000,-90.000000" false false)
  (Transformation|SetRelativeRotation _mesh_2 "0.000000,-90.000000,0.000000" false false)
  (Pawn|Components|CharacterMovement|SetMovementMode (Variables|Character|GetCharacterMovement) "MOVE_Walking" 0)
  (Actor|Tick|SetActorTickEnabled true)
  (Variables|Default|SetbIsRagdoll false)
  (CallFunction|Transitionto (Variables|Default|GetHeroState))
  (Audio|PlaySound2D "/Game/Feedback/SoundEffect/RéapparitionHero.RéapparitionHero" 1.0 1.0 0.0 0 0))

(fn StartRagdollLvl2
  (bind _mesh (Variables|Character|GetMesh))
  (CallFunction|ResetAnim)
  (Variables|Default|SetbIsMoving false)
  (Actor|Tick|SetActorTickEnabled false)
  (Pawn|Components|CharacterMovement|SetMovementMode (Variables|Character|GetCharacterMovement) "MOVE_None" 0)
  (Collision|SetCollisionEnabled (Variables|Collision|GetCapsuleComponent) "NoCollision")
  (Collision|SetCollisionProfileName _mesh "Ragdoll" true :!class /Script/Engine.PrimitiveComponent)
  (Collision|SetCollisionEnabled _mesh "QueryAndPhysics")
  (Physics|SetSimulatePhysics _mesh true)
  (Class|PrimitiveComponent|WakeAllRigidBodies _mesh)
  (Physics|AddImpulse _mesh "0.000000,0.000000,100.000000" "" true))

(fn StopragdollLvl2
  (bind _mesh (Variables|Character|GetMesh))
  (bind _capsulecomponent (Variables|Collision|GetCapsuleComponent))
  (Physics|SetSimulatePhysics _mesh false)
  (Collision|SetCollisionEnabled _mesh "NoCollision")
  (Collision|SetCollisionEnabled _capsulecomponent "QueryAndPhysics")
  (Collision|SetCollisionProfileName _capsulecomponent "Pawn" true :!class /Script/Engine.PrimitiveComponent)
  (Transformation|SetRelativeLocation (Variables|Character|GetMesh) "0.000000,0.000000,-90.000000" false false)
  (Transformation|SetRelativeRotation (Variables|Character|GetMesh) "0.000000,-90.000000,0.000000" false false)
  (Pawn|Components|CharacterMovement|SetMovementMode (Variables|Character|GetCharacterMovement) "MOVE_Walking" 0)
  (Actor|Tick|SetActorTickEnabled false)
  (Variables|Default|SetbIsRagdoll false)
  (Variables|AnimLvl1|SetAnimIsGetUp true)
  (Variables|Default|SetbIsMoving false)
  (CallFunction|DelayforGetUp))