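; Control panel actor that shows a hint when the first-person character is near and can switch BP_Hero into another state for easy mode.
; Overlap with the TriggerGreen volume sets the NearGreen flag and toggles HintWidget visibility.
; BeginPlay enables player input, though the graph has no input events and never reads NearGreen.
; ActivateEasyMode, not called within this Blueprint, calls TransitionTo on the first BP_Hero found.
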(event OnComponentBeginOverlap(TriggerGreen)
  (params (OverlappedComponent :type Primitive%20Component%20Object%20Reference) (OtherActor :type Actor%20Object%20Reference) (OtherComp :type Primitive%20Component%20Object%20Reference) (OtherBodyIndex :type Integer) (bFromSweep :type Boolean) (SweepResult :type Hit%20Result%20Structure%20%28by%20ref%29))
  (Utilities|Casting|CastToBP_FirstPersonCharacter OtherActor)
  (Variables|Default|SetbNearGreen true)
  (Rendering|SetVisibility (Variables|Default|GetHintWidget) true false))

(event OnComponentEndOverlap(TriggerGreen)
  (params (OverlappedComponent :type Primitive%20Component%20Object%20Reference) (OtherActor :type Actor%20Object%20Reference) (OtherComp :type Primitive%20Component%20Object%20Reference) (OtherBodyIndex :type Integer))
  (Utilities|Casting|CastToBP_FirstPersonCharacter OtherActor)
  (Variables|Default|SetbNearGreen false)
  (Rendering|SetVisibility (Variables|Default|GetHintWidget) false false))

(event Custom|Activate%20EasyMode
  (bind _outactors (Actor|GetAllActorsOfClass "/Game/Blueprint/Enemy/BP_Hero.BP_Hero_C"))
  (Default|Transitionto (Utilities|Array|Get(acopy) _outactors) "NewEnumerator12"))

(event EventBeginPlay
  (Input|EnableInput (Game|GetPlayerController 0)))

(fn ConstructionScript)