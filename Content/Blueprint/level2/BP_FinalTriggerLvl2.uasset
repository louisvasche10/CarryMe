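; BP_FinalTriggerLvl2 is a one-shot box trigger in level 2 that pauses the hero to show the control panel's F window.
; On first BP_Hero overlap it disables movement, switches the hero's state via TransitionTo, and calls ShowF on BP_ControlPanelLevel2.
; After a short delay, if the window is still open, it calls ByeF, restores walking and transitions the hero to another state.
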(event OnComponentBeginOverlap(Box)
  (params (OverlappedComponent :type Primitive%20Component%20Object%20Reference) (OtherActor :type Actor%20Object%20Reference) (OtherComp :type Primitive%20Component%20Object%20Reference) (OtherBodyIndex :type Integer) (bFromSweep :type Boolean) (SweepResult :type Hit%20Result%20Structure%20%28by%20ref%29))
  (bind _asbp_hero (Utilities|Casting|CastToBP_Hero OtherActor))
  (Utilities|FlowControl|DoOnce false
    (:Completed
      (Pawn|Components|CharacterMovement|SetMovementMode (Variables|/Script/Engine.Character|GetCharacterMovement _asbp_hero) "MOVE_None" 0)
      (Default|Transitionto _asbp_hero "NewEnumerator13")
      (bind _returnvalue (Actor|GetActorOfClass "/Game/Blueprint/level2/BP_ControlPanelLevel2.BP_ControlPanelLevel2_C"))
      (Default|ShowF _returnvalue)
      (Variables|/Game/Blueprint/level2/BP_ControlPanelLevel2.BP_ControlPanelLevel2_C|SetbFWindowOpen _returnvalue true)
      (Utilities|FlowControl|Delay 4.0)
      (if (== (Variables|Default|GetbWindowOpen) true)
        (bind _output_get (Variables|Default|SetAs%20BP%20Control%20Panel%20Level%202 _returnvalue))
        (Default|ByeF _returnvalue)
        (Variables|/Game/Blueprint/level2/BP_ControlPanelLevel2.BP_ControlPanelLevel2_C|SetbFWindowOpen _output_get false)
        (Pawn|Components|CharacterMovement|SetMovementMode (Variables|/Script/Engine.Character|GetCharacterMovement _asbp_hero) "MOVE_Walking" 0)
        (Default|Transitionto _asbp_hero "NewEnumerator30")))))

(event EventBeginPlay)

(event Collision|EventActorBeginOverlap
  (params (OtherActor :type Actor%20Object%20Reference)))

(event EventTick
  (params (DeltaSeconds :type Float%20%28single-precision%29)))

(fn ConstructionScript)