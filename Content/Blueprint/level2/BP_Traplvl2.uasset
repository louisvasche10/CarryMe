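; Level 2 moving-wall trap that shows a control-panel prompt (ShowF) when BP_Hero enters its detection zone.
; ActivateWallVertical slides the wall along relative X with a power-eased timeline, plays impact and reload sounds, then returns it on a second timeline.
; A gate blocks re-triggering mid-cycle, and a DoN limits activations to three.
; Tick holds a separate VInterpTo movement driven by WallMoving, which this graph never sets true.
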(event OnComponentBeginOverlap(DetectionZone)
  (params (OverlappedComponent :type Primitive%20Component%20Object%20Reference) (OtherActor :type Actor%20Object%20Reference) (OtherComp :type Primitive%20Component%20Object%20Reference) (OtherBodyIndex :type Integer) (bFromSweep :type Boolean) (SweepResult :type Hit%20Result%20Structure%20%28by%20ref%29))
  (Utilities|Casting|CastToBP_Hero OtherActor)
  (bind _returnvalue (Actor|GetActorOfClass "/Game/Blueprint/level2/BP_ControlPanelLevel2.BP_ControlPanelLevel2_C"))
  (Default|ShowF _returnvalue))

(event Custom|ActivateWallVertical
  ;[0.15 0.15 0.15 0.5] Animation du piège
  (Utilities|FlowControl|Sequence
    (:then_0
      (Utilities|FlowControl|Gate false :!label _label
        (:Exit
          (Utilities|FlowControl|DoN 3
            (:Exit
              (bind (_direction _alpha) (Timeline|Timeline PlayFromStart)
                (:Update
                  (Transformation|SetRelativeLocation (Variables|Default|GetWallMesh) (Math|Vector|Lerp(Vector) (Variables|Default|GetWallStartLocation) (Variables|Default|GetWallEndLocation) (Math|Float|Power _alpha (Utilities|Select :Index _direction :Forward 2.0 :Backward 0.5))) false false))
                (:Finished
                  (Audio|PlaySound2D "/Game/Feedback/SoundEffect/SoundLevel2/ImpactSonMur.ImpactSonMur" 1.0 1.0 0.0 0 0)
                  (Utilities|FlowControl|Delay 1.0)
                  (Audio|PlaySound2D "/Game/Feedback/SoundEffect/SoundLevel2/Rechargement_piege_mursd.Rechargement_piege_mursd" 0.6 1.0 0.0 0 0)
                  (bind _alpha_2 (Timeline|Timeline_Return PlayFromStart)
                    (:Update
                      (Utilities|FlowControl|Sequence
                        (:then_1
                          (Transformation|SetRelativeLocation (Variables|Default|GetWallMesh) (Math|Vector|Lerp(Vector) (Variables|Default|GetWallEndLocation) (Variables|Default|GetWallStartLocation) (Math|Float|Power _alpha_2 (Utilities|Select :Index "Forward" :Forward 2.0 :Backward 0.5))) false false))))
                    (:Finished
                      (goto _label Open))))))))))
    (:then_1
      (goto _label Close))))

(event EventBeginPlay
  (bind _output_get (Variables|Default|SetWallStartLocation (Variables|/Script/Engine.SceneComponent|GetRelativeLocation (Variables|Default|GetWallMesh))))
  (Variables|Default|SetWallEndLocation (Math|Vector|MakeVector (- (.X (Math|Vector|BreakVector _output_get)) (Variables|Default|GetWallMoveDistance)) (.Y (Math|Vector|BreakVector _output_get)) (.Z (Math|Vector|BreakVector _output_get)))))

(event EventTick
  (params (DeltaSeconds :type Float%20%28single-precision%29))
  (bind _wallmesh (Variables|Default|GetWallMesh))
  (if (Variables|Default|GetbWallMoving)
    (Transformation|SetRelativeLocation _wallmesh (Math|Interpolation|VInterpTo (Variables|/Script/Engine.SceneComponent|GetRelativeLocation (Variables|Default|GetWallMesh)) (Variables|Default|GetWallEndLocation) DeltaSeconds (Variables|Default|GetWallSpeed)) false false)
    (if (<= (Math|Vector|Distance(Vector) (Variables|/Script/Engine.SceneComponent|GetRelativeLocation _wallmesh) (Variables|Default|GetWallEndLocation)) 5.0)
      (Variables|Default|SetbWallMoving false)
      (Transformation|SetRelativeLocation (Variables|Default|GetWallMesh) (Variables|Default|GetWallEndLocation) false false))))

(fn ConstructionScript)