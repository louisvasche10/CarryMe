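; Level 2 control panel with three input-driven controls: button E opens the door, button A tells BP_Hero to send Debilus, and lever F triggers the vertical wall trap and a timed hero ragdoll.
; Timelines animate the controls, gated by CanUse flags that are mirrored on prompt widgets.
; Only E starts enabled; this file never enables A or F.
; The trigger overlap reveals a hint and sets NearPanel, which the inputs do not check.
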(event OnComponentBeginOverlap(TriggerGreen)
  (params (OverlappedComponent :type Primitive%20Component%20Object%20Reference) (OtherActor :type Actor%20Object%20Reference) (OtherComp :type Primitive%20Component%20Object%20Reference) (OtherBodyIndex :type Integer) (bFromSweep :type Boolean) (SweepResult :type Hit%20Result%20Structure%20%28by%20ref%29))
  ;[0.15 0.15 0.15 0.5] le panel que le joueur est là donc le rend accessible
  (Utilities|Casting|CastToBP_FirstPersonCharacter OtherActor)
  (Variables|Default|SetRefHero 0)
  (Variables|Default|SetNearPanel true)
  (Rendering|SetVisibility (Variables|Default|GetHintWidget) true false))

(event Custom|ShowA)

(event Custom|ShowF)

(event Custom|ByeF)

(event Custom|ByeA)

(event Custom|Bye%20E)

(event Input|EnhancedActionEvents|EnhancedInputActionIA_Interact
  (params (ActionValue :type Boolean) (ElapsedSeconds :type Float%20%28double-precision%29) (TriggeredSeconds :type Float%20%28double-precision%29) (InputAction :type Input%20Action%20Object%20Reference :default "/Game/Input/Actions/IA_Interact.IA_Interact"))
  (:Started
    ;[0.15 0.15 0.15 0.5] la porte s'ouvre quand on appuie sur E
    (if (Variables|Default|GetCanUse_E)
      (Audio|SpawnSound2D "/Game/Feedback/SoundEffect/ClickBouton.ClickBouton" 1.0 1.0 0.0 0)
      (bind _press (Timeline|TL_ButtonPress PlayFromStart)
        (:Update
          (Transformation|SetRelativeLocation (Variables|Default|GetBtn_E) (Math|Vector|Lerp(Vector) (Variables|Default|GetBtnE_StartLocation) (+ (Variables|Default|GetBtnE_StartLocation) "0.000000,0.000000,-8.000000") _press) false false))
        (:Finished
          (Default|OpenDoorLvl2 (Variables|Default|GetRefDoor))
          (CallFunction|ByeE)
          (Variables|Default|SetCanUse_E false)
          (CallFunction|UpdateInputLettersVisual))))))

(event Input|EnhancedActionEvents|EnhancedInputActionIA_SendDebilus
  (params (ActionValue :type Boolean) (ElapsedSeconds :type Float%20%28double-precision%29) (TriggeredSeconds :type Float%20%28double-precision%29) (InputAction :type Input%20Action%20Object%20Reference :default "/Game/Input/Actions/IA_SendDebilus.IA_SendDebilus"))
  ;[0.15 0.15 0.15 0.5] send debilus quand on appuie sur A
  (:Started
    (if (Variables|Default|GetCanUse_A)
      (Audio|SpawnSound2D "/Game/Feedback/SoundEffect/ClickBouton.ClickBouton" 1.0 1.0 0.0 0)
      (bind _press (Timeline|Timeline PlayFromStart)
        (:Update
          (Transformation|SetRelativeLocation (Variables|Default|GetBtn_A) (Math|Vector|Lerp(Vector) (Variables|Default|GetBtnA_StartLocation) (+ (Variables|Default|GetBtnA_StartLocation) "0.000000,0.000000,-8.000000") _press) false false)
          (if (Variables|Default|GetCanUse_A)
            (bind _returnvalue (Actor|GetActorOfClass "/Game/Blueprint/Enemy/BP_Hero.BP_Hero_C"))
            (Default|SendDebilus _returnvalue)
            (Variables|Default|SetCanUse_A false)
            (CallFunction|UpdateInputLettersVisual)))))))

(event Input|EnhancedActionEvents|EnhancedInputActionIA_F
  (params (ActionValue :type Boolean) (ElapsedSeconds :type Float%20%28double-precision%29) (TriggeredSeconds :type Float%20%28double-precision%29) (InputAction :type Input%20Action%20Object%20Reference :default "/Game/Input/Actions/IA_F.IA_F"))
  (:Started
    (if (Variables|Default|GetCanUse_F)
      (Audio|SpawnSound2D "/Game/Feedback/SoundEffect/ClickBouton.ClickBouton" 1.0 1.0 0.0 0)
      (bind _alpha (Timeline|Timeline_0 PlayFromStart)
        (:Update
          (Transformation|SetRelativeRotation (Variables|Default|GetLevier) (Math|Rotator|Lerp(Rotator) (Variables|Default|GetLevierStartLocation) (Math|Rotator|CombineRotators (Variables|Default|GetLevierStartLocation) "-60.000000,0.000000,0.000000") _alpha) false false))
        (:Finished
          (if (Variables|Default|GetCanUse_F)
            (Utilities|FlowControl|DoOnce false
              (:Completed
                (CallFunction|UpdateInputLettersVisual)
                (Default|ActivateWallVertical (Variables|Default|GetRef_BpTrapLvl2))
                (bind _returnvalue (Actor|GetActorOfClass "/Game/Blueprint/Enemy/BP_Hero.BP_Hero_C"))
                (Utilities|FlowControl|Delay 1.0)
                (Default|StartRagdollLvl2 _returnvalue)
                (Variables|Default|SetCanUse_F false)
                (CallFunction|UpdateInputLettersVisual)
                (Utilities|FlowControl|Delay 6.0)
                (Default|StopragdollLvl2 _returnvalue)))))))))

(event EventBeginPlay
  (Variables|Default|SetLevierStartLocation (Variables|/Script/Engine.SceneComponent|GetRelativeRotation (Variables|Default|GetLevier)))
  (Variables|Default|SetBtnA_StartLocation (Variables|/Script/Engine.SceneComponent|GetRelativeLocation (Variables|Default|GetBtn_A)))
  (Variables|Default|SetBtnE_StartLocation (Variables|/Script/Engine.SceneComponent|GetRelativeLocation (Variables|Default|GetBtn_E)))
  (Input|EnableInput (Game|GetPlayerController 0))
  (Variables|Default|SetCanUse_A false)
  (Variables|Default|SetCanUse_F false)
  (Variables|Default|SetCanUse_E true)
  (CallFunction|UpdateInputLettersVisual))

(fn ConstructionScript)

(fn UpdateInputLettersVisual
  (Utilities|FlowControl|Sequence
    (:then_0
      (bind _aswbp_level_2input_a (Utilities|Casting|CastToWBP_Level2InputA (UserInterface|GetUserWidgetObject (Variables|Default|GetWBP_A))))
      (if (== (Variables|Default|GetCanUse_A) false)
        (Default|SetInputActive _aswbp_level_2input_a false)
        (else
          (Default|SetInputActive _aswbp_level_2input_a true))))
    (:then_1
      (bind _aswbp_level_2input_f (Utilities|Casting|CastToWBP_Level2InputF (UserInterface|GetUserWidgetObject (Variables|Default|GetWBP_F))))
      (if (== false (Variables|Default|GetCanUse_F))
        (Default|IsActiveF _aswbp_level_2input_f false)
        (else
          (Default|IsActiveF _aswbp_level_2input_f true))))
    (:then_2
      (bind _aswbp_level_2input_e (Utilities|Casting|CastToWBP_Level2InputE (UserInterface|GetUserWidgetObject (Variables|Default|GetWBP_E))))
      (if (== false (Variables|Default|GetCanUse_E))
        (Default|NewFunction _aswbp_level_2input_e false)
        (else
          (Default|NewFunction _aswbp_level_2input_e true))))))