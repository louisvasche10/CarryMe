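; Level 2 double wooden door that unlocks and swings open when OpenDoorLvl2 is called.
; If still locked, the event starts the opening and plays an unlock sound after a short delay.
; Tick eases both leaves toward their target yaws with RInterpTo, clearing IsLock once both are nearly there.
; DoorOpenTrue, meant to tell the hero, is set while the leaves are still moving; ShouldGetOpen is never reset.
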(event Custom|OpenDoorLvl2
  ;[0.15 0.15 0.15 0.5] La porte s'ouvre
  (if (== (Variables|Default|GetbIsLock) true)
    (Variables|Default|SetShouldGetOpen? true)
    (Utilities|FlowControl|Delay 0.2)
    (Audio|PlaySound2D "/Game/Feedback/SoundEffect/SoundLevel1/SW_Porte_qui_se_déverouille.SW_Porte_qui_se_déverouille" 1.0 1.0 0.0 0 0)))

(event EventTick
  (params (DeltaSeconds :type Float%20%28single-precision%29))
  (bind _sm_door_wood_left (Variables|Components|GetSM_door_wood_left))
  (bind _sm_door_wood_right (Variables|Components|GetSM_door_wood_right))
  ;[0.15 0.15 0.15 0.5] La porte s'ouvre
  (if (== (Variables|Default|GetShouldGetOpen?) true)
    (if true
      (Transformation|SetRelativeRotation _sm_door_wood_left (Math|Interpolation|RInterpTo (Variables|/Script/Engine.SceneComponent|GetRelativeRotation _sm_door_wood_left) (Math|Rotator|MakeRotator 0.0 0.0 (Variables|Default|GetOpenAngleL)) DeltaSeconds (Variables|Default|GetOpenSeed)) false false)
      (Transformation|SetRelativeRotation _sm_door_wood_right (Math|Interpolation|RInterpTo (Variables|/Script/Engine.SceneComponent|GetRelativeRotation _sm_door_wood_right) (Math|Rotator|MakeRotator 0.0 0.0 (Variables|Default|GetOpenAngleR)) DeltaSeconds (Variables|Default|GetOpenSeed)) false false)
      (if (and (Math|Float|NearlyEqual(Float) (.Yaw (Math|Rotator|BreakRotator (Variables|/Script/Engine.SceneComponent|GetRelativeRotation _sm_door_wood_left))) (Variables|Default|GetOpenAngleL) 1.0) (Math|Float|NearlyEqual(Float) (.Yaw (Math|Rotator|BreakRotator (Variables|/Script/Engine.SceneComponent|GetRelativeRotation _sm_door_wood_right))) (Variables|Default|GetOpenAngleR) 1.0))
        (Variables|Default|SetbIsLock false)
        (else
          ;;[0.15 0.15 0.15 0.5] Dire au héro que la porte est ouverte.
          (Variables|Default|SetDoorOpenTrue? true))))))

(fn ConstructionScript)