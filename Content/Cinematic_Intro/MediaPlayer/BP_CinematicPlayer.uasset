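; Cinematic player, placed per level, that plays a configured media source with its sound in a widget, then moves on to a chosen level.
; BeginPlay binds the media end event, and a five-second timer shows a press-space prompt that enables skipping straight to NextLevel.
; Generated handlers either fade to black and open NextLevel or, when EndAction is set, show an end-CG widget for a set duration before the main menu.
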(event Custom|EnableSkip
  (Variables|Default|SetbCanSkip true)
  (bind _returnvalue (UserInterface|CreateWidget "/Game/Widget/Scene_Widget/WBP_PressSpace.WBP_PressSpace_C"))
  (Variables|Default|SetWBP_PRESSSPACE _returnvalue)
  (UserInterface|Viewport|AddtoViewport _returnvalue 0))

(event Custom|FinishCinematic
  (bind _wbp_pressspace (Variables|Default|GetWBP_PRESSSPACE))
  (Utilities|IsValid _wbp_pressspace
    (:Is%20Valid
      (Widget|RemovefromParent _wbp_pressspace)
      (Game|OpenLevel(byName) (Variables|Default|GetNextLevel)))))

(event Custom|EndWidget
  (bind _returnvalue (UserInterface|CreateWidget "/Game/Cinematic_Intro/WBP/WBP_EndCG.WBP_EndCG_C"))
  (bind _output_get (Variables|Default|SetWBP_EndCG _returnvalue))
  (UserInterface|Viewport|AddtoViewport _returnvalue 0)
  (Utilities|FlowControl|Delay (Variables|Default|GetEndCGduration))
  (Development|PrintString "on attend")
  (Widget|RemovefromParent _output_get)
  (bind _returnvalue_2 (UserInterface|CreateWidget "/Game/Widget/GameMenu/WBP_MainMenu.WBP_MainMenu_C"))
  (Variables|Default|SetWBP_MM _returnvalue_2)
  (UserInterface|Viewport|AddtoViewport _returnvalue_2 0))

(event Input|EnhancedActionEvents|EnhancedInputActionIA_Espace
  (params (ActionValue :type Boolean) (ElapsedSeconds :type Float%20%28double-precision%29) (TriggeredSeconds :type Float%20%28double-precision%29) (InputAction :type Input%20Action%20Object%20Reference :default "/Game/Input/Actions/IA_Espace.IA_Espace"))
  (if (Variables|Default|GetbCanSkip)
    (CallFunction|FinishCinematic)))

(event EventBeginPlay
  (bind _mediaplayer_cine (Variables|Default|GetMediaPlayer_Cine))
  ;[0.15 0.15 0.15 0.5] choix dans les levels des cinématiques qu'on lance et de la source de son qui suit avec et quand la cinématique se finit on passe au level selectionné dans le level
  (Input|EnableInput (Game|GetPlayerController 0))
  (bind _returnvalue (UserInterface|CreateWidget (Variables|Default|GetWidgetClass) (Game|GetPlayerController 0)))
  (UserInterface|Viewport|AddtoViewport _returnvalue 0)
  (Media|MediaPlayer|OpenSource _mediaplayer_cine (Variables|Default|GetMedialSource_Cine))
  (Media|MediaSoundComponent|SetMediaPlayer (Variables|Default|GetMediaSoundComp) _mediaplayer_cine)
  (Media|MediaPlayer|BindEventtoOnEndReached _mediaplayer_cine (EventDispatchers|CreateEvent :!event BPCinematicPlayerAutoGenFunc))
  (Variables|Default|SetbCanSkip false)
  (Utilities|Time|SetTimerbyEvent (delegate Custom|EnableSkip) 5.0))

(fn ConstructionScript)

(fn BPCinematicPlayerAutoGenFunc
  (bind _wbp_pressspace (Variables|Default|GetWBP_PRESSSPACE))
  ;[0.15 0.15 0.15 0.5] quand on clique sur le btn le wbp dégrade sur une image noir et le level qu'on inscrit dans les levels se lance
  (if (Variables|Default|GetEndAction)
    (CallFunction|EndWidget)
    (else
      (Utilities|IsValid _wbp_pressspace
        (:Is%20Valid
          (Widget|RemovefromParent _wbp_pressspace)
          (bind _returnvalue (UserInterface|CreateWidget "/Game/Widget/WBP_FadeToBlack.WBP_FadeToBlack_C"))
          (Variables|Default|SetIN _returnvalue)
          (UserInterface|Viewport|AddtoViewport _returnvalue 0)
          (EventDispatchers|BindEventtoOnFadeinComplete (Variables|Default|GetIN) (EventDispatchers|CreateEvent :!event BPCinematicPlayerAutoGenFunc1))
          (Default|PlayFadein (Variables|Default|GetIN)))))))

(fn BPCinematicPlayerAutoGenFunc1
  (if (Variables|Default|GetEndAction)
    (CallFunction|EndWidget)
    (else
      (Game|OpenLevel(byName) (Variables|Default|GetNextLevel)))))